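; BP_Planet is a planet actor that sizes its mesh from a radius given in meters.
; The construction script converts the radius to Unreal units and uniformly scales PlanetMesh by that value divided by the component's X bounds extent.
; It then sets the mesh's relative Z location.
; The event graph holds only disabled placeholder events, so the Blueprint adds no runtime logic.
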(event EventBeginPlay)

(event Collision|EventActorBeginOverlap
  (params (OtherActor :type Actor%20Object%20Reference)))

(event EventTick
  (params (DeltaSeconds :type Float%20%28single-precision%29)))

(fn ConstructionScript
  (bind _planetmesh (Variables|Default|GetPlanetMesh))
  (bind _output_get (Variables|Default|SetRadiusInUnits (* (Variables|Default|GetRadiusInMeters) 1e+02)))
  (Transformation|SetWorldScale3D _planetmesh (Math|Conversions|ToVector(Float) (/ _output_get (.x (.BoxExtent (Collision|GetComponentBounds (Variables|Default|GetPlanetMesh)))))))
  (Transformation|SetRelativeLocation _planetmesh (Math|Vector|MakeVector 0.0 0.0 (stale _result)) false false))